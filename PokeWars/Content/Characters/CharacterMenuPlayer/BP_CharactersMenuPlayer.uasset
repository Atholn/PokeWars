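; BP_CharactersMenuPlayer is the pawn behind the character menu screens, showing the characters menu widget on BeginPlay.
; Two functions swap between the characters menu and the new character menu, removing the current widget and creating the other fresh.
; Opening the new character menu also calls CreatePokemonList on the controlled pawn, filling that widget with names and profile images from the BPCPokemons component.
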(event Custom|CreatePokemonList
  (bind _pokemons (Default|GetPokemons (Variables|Default|GetBPC_Pokemons)))
  (bind _output_get (Variables|Default|SetPokeomons _pokemons))
  (for _array_element _output_get
    (Default|AddPokemontoListUI (Variables|Default|GetNewCharackterMenuWidget) (.Name (Utilities|Struct|BreakPokemon _array_element)) (.ProfileImage (Utilities|Struct|BreakPokemon _array_element)))))

(event EventBeginPlay
  (bind _returnvalue (UserInterface|CreateWidget "/Game/UI/CharactersMenu/WBP_CharactersMenu.WBP_CharactersMenu_C"))
  (UserInterface|Viewport|AddtoViewport _returnvalue 0)
  (Variables|Default|SetCharacktersMenuWidget _returnvalue))

(fn ConstructionScript)

(fn GotoNewCharacterMenu
  (Widget|RemovefromParent (Variables|Default|GetCharacktersMenuWidget))
  (bind _returnvalue (UserInterface|CreateWidget "/Game/UI/CharactersMenu/WBP_NewCharacterMenu.WBP_NewCharacterMenu_C"))
  (UserInterface|Viewport|AddtoViewport _returnvalue 0)
  (bind _asbp_characters_menu_player (Utilities|Casting|CastToBP_CharactersMenuPlayer (Pawn|GetControlledPawn (Game|GetPlayerController 0))))
  (Variables|Default|SetNewCharackterMenuWidget _returnvalue)
  (CallFunction|CreatePokemonList _asbp_characters_menu_player))

(fn GotoCharactersMenu
  (Widget|RemovefromParent (Variables|Default|GetNewCharackterMenuWidget))
  (bind _returnvalue (UserInterface|CreateWidget "/Game/UI/CharactersMenu/WBP_CharactersMenu.WBP_CharactersMenu_C"))
  (UserInterface|Viewport|AddtoViewport _returnvalue 0)
  (Variables|Default|SetCharacktersMenuWidget _returnvalue))