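; BPC_Stats is a character stats component that tracks health and level data and destroys its owner when health runs out.
; Damage and healing adjust HP, capped at the maximum, and return death status on damage.
; Health changes push to the HUD widget by casting the owner to BP_Character.
; Setters load health and level values, while energy, XP gain, level-up and max-health increase functions are empty stubs.
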(event EventBeginPlay)

(fn DecreseHealth
  (params (Damage :type Float%20%28double-precision%29))
  (if (> (Variables|Health|GetHP) Damage)
    (Variables|Health|SetHP (- (Variables|Health|GetHP) Damage))
    (Development|PrintString "Hello")
    (Health|SetHpinUI)
    (return false)
    (else
      (Variables|Health|SetHP 0.0)
      (Actor|DestroyActor (Components|GetOwner))
      (Health|SetHpinUI)
      (return true))))

(fn IncreaseMaxHealth
  (params (HealthIncremention :type Float%20%28double-precision%29)))

(fn DevreaseEnergy
  (params (StaminaDecrease :type Float%20%28double-precision%29)))

(fn IncreaseMaxEnergy
  (params (AddStamina :type Float%20%28double-precision%29)))

(fn IncreaseHealth
  (params (AddedHealth :type Float%20%28double-precision%29))
  (Variables|Health|SetHP (+ (Variables|Health|GetHP) AddedHealth))
  (if (> (Variables|Health|GetHP) (Variables|Health|GetHPMax))
    (Variables|Health|SetHP (Variables|Health|GetHPMax)))
  (Health|SetHpinUI))

(fn IncreaseEnergy
  (params (AddedStamina :type Float%20%28double-precision%29)))

(fn IncreaseXP
  (params (AddedXP :type Float%20%28double-precision%29)))

(fn IncreaseLevel
  (params (AddedLevel :type Integer) (XP :type Float%20%28double-precision%29)))

(fn SetLevelStats
  (params (LevelStats :type Level%20Stats%20Structure))
  (bind (_level _xp _xpmax) (Utilities|Struct|BreakLevelStats LevelStats))
  (Variables|XP|SetLevel _level)
  (Variables|XP|SetXP _xp)
  (Variables|XP|SetMaxXP _xpmax))

(fn SetHealthStats
  (params (HP :type Float%20%28double-precision%29) (HPMax :type Float%20%28double-precision%29))
  (Variables|Health|SetHP HP)
  (Variables|Health|SetHPMax HPMax)
  (Health|SetHpinUI))

(fn SetHpinUI
  (bind _asbp_character (Utilities|Casting|CastToBP_Character (Components|GetOwner)))
  (Default|SetHp (Variables|/Game/Characters/Player/BP_Character.BP_Character_C|GetHUD%20Widget _asbp_character) (Variables|Health|GetHP) (Variables|Health|GetHPMax)))