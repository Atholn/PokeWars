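; Component that serves as a hard-coded catalog of Pokemon data, split into a main roster and a mob list.
; BeginPlay fills Pokemons with Jolteon, Flareon and Vaporeon, and PokemonMobs with Eevee.
; Each entry is a struct with a fixed GUID, enum-derived name, description, and profile images and meshes for base, attack, defense and speed variants, though Eevee lacks an attack image.
; Two getters expose the arrays.
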(event EventBeginPlay
  (bind _returnvalue (Utilities|Enum|LiteralenumPokemonEnum "NewEnumerator0"))
  (bind _returnvalue_2 (Utilities|Enum|LiteralenumPokemonEnum "NewEnumerator2"))
  (bind _returnvalue_3 (Utilities|Enum|LiteralenumPokemonEnum "NewEnumerator1"))
  (bind _returnvalue_4 (Utilities|Enum|LiteralenumPokemonEnum "NewEnumerator3"))
  (bind _pokemons (Variables|Default|GetPokemons))
  ;[1 1 1] Jolteon
  (Utilities|Array|Add _pokemons (Utilities|Struct|MakePokemon (.OutGuid (Class|KismetGuidLibrary|ParseStringtoGuid "3ab58d56-b26f-4a1e-bf00-57025d9dd7ad")) (Utilities|String|EnumtoString _returnvalue) "Jolteon Description" _returnvalue "NewEnumerator0" "" (Utilities|Struct|MakeProfileImages "/Game/Assets/PokemonProfileImages/JolteonProfileImage.JolteonProfileImage" "/Game/Assets/PokemonProfileImages/JolteonAttackProfile.JolteonAttackProfile" "/Game/Assets/PokemonProfileImages/JolteonDefenseProfile.JolteonDefenseProfile" "/Game/Assets/PokemonProfileImages/JolteonSpeedProfile.JolteonSpeedProfile") (Utilities|Struct|MakePokemonMeshes "/Game/Models/Jolteon/Base/JolteonBase.JolteonBase" "/Game/Models/Jolteon/Attack/JolteonAttack.JolteonAttack" "/Game/Models/Jolteon/Defense/JolteonDefense.JolteonDefense" "/Game/Models/Jolteon/Speed/JolteonSpeed.JolteonSpeed")))
  ;[1 1 1] Flareon
  (Utilities|Array|Add _pokemons (Utilities|Struct|MakePokemon (.OutGuid (Class|KismetGuidLibrary|ParseStringtoGuid "acb73c13-ed2d-4560-b357-b1d55f8ec1df")) (Utilities|String|EnumtoString _returnvalue_3) "Flareon Description" _returnvalue_3 "NewEnumerator1" "" (Utilities|Struct|MakeProfileImages "/Game/Assets/PokemonProfileImages/FlareonProfileImage.FlareonProfileImage" "/Game/Assets/PokemonProfileImages/FlareonAttackProfile.FlareonAttackProfile" "/Game/Assets/PokemonProfileImages/FlareonDefenseProfile.FlareonDefenseProfile" "/Game/Assets/PokemonProfileImages/FlareonSpeedProfile.FlareonSpeedProfile") (Utilities|Struct|MakePokemonMeshes "/Game/Models/Flareon/Base/FlareonBase.FlareonBase" "/Game/Models/Flareon/Attack/FlareonAttack.FlareonAttack" "/Game/Models/Flareon/Defense/FlareonDefense.FlareonDefense" "/Game/Models/Flareon/Speed/FlareonSpeed.FlareonSpeed")))
  ;[1 1 1] Vaporeon
  (Utilities|Array|Add _pokemons (Utilities|Struct|MakePokemon (.OutGuid (Class|KismetGuidLibrary|ParseStringtoGuid "3e62f452-bec7-487a-b6a4-44cbf5e15d30")) (Utilities|String|EnumtoString _returnvalue_2) "Vaporeon Description" _returnvalue_2 "NewEnumerator2" "" (Utilities|Struct|MakeProfileImages "/Game/Assets/PokemonProfileImages/VaporeonProfileImage.VaporeonProfileImage" "/Game/Assets/PokemonProfileImages/VaporeonAttackProfile.VaporeonAttackProfile" "/Game/Assets/PokemonProfileImages/VaporeonDefenseProfile.VaporeonDefenseProfile" "/Game/Assets/PokemonProfileImages/VaporeonSpeedProfile.VaporeonSpeedProfile") (Utilities|Struct|MakePokemonMeshes "/Game/Models/Vaporeon/Base/VaporeonBase.VaporeonBase" "/Game/Models/Vaporeon/Attack/VaporeonAttack.VaporeonAttack" "/Game/Models/Vaporeon/Defense/VaporeonDefense.VaporeonDefense" "/Game/Models/Vaporeon/Speed/VaporeonSpeed.VaporeonSpeed")))
  (Utilities|Array|Add (Variables|Default|GetPokemonMobs) (Utilities|Struct|MakePokemon (.OutGuid (Class|KismetGuidLibrary|ParseStringtoGuid "1daaff93-7739-4107-9169-ad8e0d65d187")) (Utilities|String|EnumtoString _returnvalue_4) "Eevee description" _returnvalue_4 "NewEnumerator3" "" (Utilities|Struct|MakeProfileImages "/Game/Assets/PokemonProfileImages/EeeveeProfileImage.EeeveeProfileImage" 0 "/Game/Assets/PokemonProfileImages/EeeveeProfileImage.EeeveeProfileImage" "/Game/Assets/PokemonProfileImages/EeeveeProfileImage.EeeveeProfileImage") (Utilities|Struct|MakePokemonMeshes "/Game/Models/Eevee/Base/eevee.eevee" "/Game/Models/Eevee/Attack/eeveeAttack.eeveeAttack" "/Game/Models/Eevee/Defense/eeveeDefense.eeveeDefense" "/Game/Models/Eevee/Speed/eeveeSpeed.eeveeSpeed"))))

(fn GetPokemons
  (return (Variables|Default|GetPokemons)))

(fn GetPokemonMobs
  (return (Variables|Default|GetPokemonMobs)))