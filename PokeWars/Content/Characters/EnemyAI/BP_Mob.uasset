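; Enemy mob character for a Pokémon-themed game, with health, target info, death and a stealth back-assassination reaction.
; SetTargetInfo looks up the Pokémon in PokemonsSystem's mob list to fill BPCTarget, and initializes health in BPCStats.
; Damage goes through BPCStats, which can trigger death: input off, ragdoll, delayed destroy.
; StealthBackAssasin plays an Eevee montage, starts a delayed ragdoll without destroying the actor, and returns mesh location and actor rotation.
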(event Custom|Die
  ;[1 1 1] Die
  (Input|DisableInput 0)
  (Physics|SetSimulatePhysics (Variables|Character|GetMesh) true)
  (Utilities|FlowControl|Delay 5.0)
  (Actor|DestroyActor))

(event Custom|Ragdoll
  (Utilities|FlowControl|Delay 2.5)
  (Physics|SetSimulatePhysics (Variables|Character|GetMesh) true))

(event Collision|EventActorBeginOverlap
  (params (OtherActor :type Actor%20Object%20Reference)))

(event EventTick
  (params (DeltaSeconds :type Float%20%28single-precision%29)))

(event Game|Damage|EventAnyDamage
  (params (Damage :type Float%20%28single-precision%29) (DamageType :type Damage%20Type%20Object%20Reference) (InstigatedBy :type Controller%20Object%20Reference) (DamageCauser :type Actor%20Object%20Reference))
  ;[1 1 1] Damage
  (bind _isdead (Default|DecreseHealth (Variables|Default|GetBPC_Stats) Damage))
  (if _isdead
    (CallFunction|Die)))

(event EventBeginPlay)

(fn ConstructionScript)

(fn SetTargetInfo
  (params (Pokemon :type PokemonEnum%20Enum :default "NewEnumerator0"))
  (bind _returnvalue (Actor|GetActorOfClass "/Game/Characters/PokemonsSystem.PokemonsSystem_C"))
  (bind _pokemonmobs (Default|GetPokemonMobs (Variables|/Game/Characters/PokemonsSystem.PokemonsSystem_C|GetBPC_Pokemons _returnvalue)))
  (bind _array_element (Utilities|Array|ForEachLoopwithBreak _pokemonmobs :!label _label)
    (:LoopBody
      (if (Utilities|Enum|Equal(Enum) Pokemon (.Pokemon (Utilities|Struct|BreakPokemon _array_element)))
        (Variables|Default|SetPokemon _array_element)
        (goto _label Break)))
    (:Completed
      (Default|SetBaseInfo (Variables|Default|GetBPC_Target) (.ProfileBaseImage (Utilities|Struct|BreakProfileImages (.ProfileImages (Utilities|Struct|BreakPokemon _array_element)))) (.Name (Utilities|Struct|BreakPokemon _array_element)) 1 0.0 0.0 0.0 0.0)
      (Default|SetHealthStats (Variables|Default|GetBPC_Stats) 1e+02 1e+02))))

(fn StealthBackAssasin
  (Animation|PlayAnimMontage "/Game/Animations/Eevee/BaseMode/Attack/AM_eevee_Anim_Attack1_Montage.AM_eevee_Anim_Attack1_Montage" 1.0 "None")
  (CallFunction|Ragdoll)
  (return (Transformation|GetWorldLocation (Variables|Character|GetMesh)) (Transformation|GetActorRotation)))