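; Targeting component for characters and mobs that holds display info, the owner's current target and a list of actors targeting the owner.
; Player targeting traces under the cursor, accepts only living mobs, moves the back-reference and decal to the new target and updates the target panel.
; RefreshReferences pushes HP changes or death to the HUDs of targeting characters.
; Mob targeting is empty and player-on-player targeting remains a todo.
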(event EventBeginPlay)

(event EventTick
  (params (DeltaSeconds :type Float%20%28single-precision%29)))

(fn SetBaseInfo
  (params (ProfileImage :type Texture%202D%20Object%20Reference) (Name :type String) (Level :type Integer) (HP :type Float%20%28double-precision%29) (HPMax :type Float%20%28double-precision%29) (Energy :type Float%20%28double-precision%29) (EnergyMax :type Float%20%28double-precision%29))
  (Variables|Default|SetTargetImage ProfileImage)
  (Variables|Default|SetTargetName Name)
  (Variables|Default|SetTargetLevel Level)
  (Variables|Default|SetHP HP)
  (Variables|Default|SetHPMax HPMax)
  (Variables|Default|SetEnergy Energy)
  (Variables|Default|SetEnergy%20Max EnergyMax))

(fn SetTargetforPlayer
  (params (UiPlayWidget :type WB%20HUD%20Object%20Reference))
  (bind _returnvalue (Components|GetOwner))
  (if (Utilities|IsValid (Variables|Default|GetCharacterTarget))
    (bind _asbp_character (Utilities|Casting|CastToBP_Character (Variables|Default|GetCharacterTarget))
      (:then
        (CallFunction|DeleteReference (Variables|/Game/Characters/Player/BP_Character.BP_Character_C|GetBPC_Target _asbp_character) _returnvalue))
      (:CastFailed
        (bind _asbp_mob (Utilities|Casting|CastToBP_Mob (Variables|Default|GetCharacterTarget))
          (:then
            (Default|HideDecal _asbp_mob)
            (CallFunction|DeleteReference (Variables|/Game/Characters/EnemyAI/BP_Mob.BP_Mob_C|GetBPC_Target _asbp_mob) _returnvalue))
          (:CastFailed
            _)))))
  (bind _output_get (Variables|Default|SetCharacterTarget (.HitActor (Collision|BreakHitResult (.HitResult (Game|Player|GetHitResultUnderCursorbyChannel (Game|GetPlayerController 0) "TraceTypeQuery1" true))))))
  (bind _asbp_mob_2 (Utilities|Casting|CastToBP_Mob _output_get)
    (:then
      (if (not (Variables|/Game/Characters/BPC_Stats.BPC_Stats_C|GetIsDead (Variables|/Game/Characters/EnemyAI/BP_Mob.BP_Mob_C|GetBPC_Stats _asbp_mob_2)))
        (CallFunction|AddReference (Variables|/Game/Characters/EnemyAI/BP_Mob.BP_Mob_C|GetBPC_Target _asbp_mob_2) (Components|GetOwner))
        (Default|SetTargetInfo UiPlayWidget (Variables|BPC_Target_C|GetTargetImage (Variables|/Game/Characters/EnemyAI/BP_Mob.BP_Mob_C|GetBPC_Target _asbp_mob_2)) (Variables|BPC_Target_C|GetTargetName (Variables|/Game/Characters/EnemyAI/BP_Mob.BP_Mob_C|GetBPC_Target _asbp_mob_2)) (Variables|BPC_Target_C|GetTargetLevel (Variables|/Game/Characters/EnemyAI/BP_Mob.BP_Mob_C|GetBPC_Target _asbp_mob_2)) (Variables|/Game/Characters/BPC_Stats.BPC_Stats_C|GetHP (Variables|/Game/Characters/EnemyAI/BP_Mob.BP_Mob_C|GetBPC_Stats _asbp_mob_2)) (Variables|/Game/Characters/BPC_Stats.BPC_Stats_C|GetHPMax (Variables|/Game/Characters/EnemyAI/BP_Mob.BP_Mob_C|GetBPC_Stats _asbp_mob_2)))
        (Default|ShowDecal _asbp_mob_2)
        (else
          (Default|HideTargetPanel UiPlayWidget :!label _label))))
    (:CastFailed
      ;[1 1 1] cast to other player / todo
      (Variables|Default|SetCharacterTarget 0)
      (goto _label))))

(fn SetTargetforMob)

(fn ClearTarget
  (Variables|Default|SetCharacterTarget 0))

(fn UpdateTarget
  (params (PlayerUI :type WB%20HUD%20Object%20Reference))
  (bind _asbp_mob (Utilities|Casting|CastToBP_Mob (Variables|Default|GetCharacterTarget)))
  (Default|SetTargetInfo PlayerUI (Variables|BPC_Target_C|GetTargetImage (Variables|/Game/Characters/EnemyAI/BP_Mob.BP_Mob_C|GetBPC_Target _asbp_mob)) (Variables|BPC_Target_C|GetTargetName (Variables|/Game/Characters/EnemyAI/BP_Mob.BP_Mob_C|GetBPC_Target _asbp_mob)) (Variables|BPC_Target_C|GetTargetLevel (Variables|/Game/Characters/EnemyAI/BP_Mob.BP_Mob_C|GetBPC_Target _asbp_mob)) (Variables|/Game/Characters/BPC_Stats.BPC_Stats_C|GetHP (Variables|/Game/Characters/EnemyAI/BP_Mob.BP_Mob_C|GetBPC_Stats _asbp_mob)) (Variables|/Game/Characters/BPC_Stats.BPC_Stats_C|GetHPMax (Variables|/Game/Characters/EnemyAI/BP_Mob.BP_Mob_C|GetBPC_Stats _asbp_mob))))

(fn AddReference
  (params (ActorWhoTargeting :type Actor%20Object%20Reference))
  (bind _targetsreferences (Variables|Default|GetTargetsReferences))
  (Utilities|Array|Add _targetsreferences ActorWhoTargeting)
  (Development|PrintString (Utilities|String|Append "length  after add" (Utilities|String|ToString(Integer) (Utilities|Array|Length _targetsreferences)) "Owner" (Utilities|GetObjectName (Components|GetOwner)) "Actor whos targeting" (Utilities|GetObjectName ActorWhoTargeting)) true true "(R=0.000000,G=0.660000,B=1.000000,A=1.000000)" 3e+01)
  (return))

(fn DeleteReference
  (params (NewParam :type Actor%20Object%20Reference))
  (bind _returnvalue (Utilities|GetObjectName NewParam))
  (bind _returnvalue_2 (Components|GetOwner))
  (bind _targetsreferences (Variables|Default|GetTargetsReferences))
  (bind _returnvalue_3 (Utilities|GetObjectName _returnvalue_2))
  (Development|PrintString (Utilities|String|Append "length  before delete: " (Utilities|String|ToString(Integer) (Utilities|Array|Length _targetsreferences)) "   Delete fro m Owner : " _returnvalue_3 "       Actor whos targeting" _returnvalue) true true "(R=0.000000,G=0.660000,B=1.000000,A=1.000000)" 3e+01)
  (Utilities|Array|RemoveItem _targetsreferences NewParam)
  (Development|PrintString (Utilities|String|Append "length  after delete: " (Utilities|String|ToString(Integer) (Utilities|Array|Length _targetsreferences)) "   Delete fro m Owner : " _returnvalue_3 "       Actor whos targeting" _returnvalue) true true "(R=0.000000,G=0.660000,B=1.000000,A=1.000000)" 3e+01)
  (return))

(fn RefreshReferences
  (params (HP :type Float%20%28double-precision%29) (HPMax :type Float%20%28double-precision%29) (IsDead :type Boolean))
  (for _array_element (Variables|Default|GetTargetsReferences)
    (bind _asbp_character (Utilities|Casting|CastToBP_Character _array_element))
    (if IsDead
      (Default|HideTargetPanel (Variables|/Game/Characters/Player/BP_Character.BP_Character_C|GetHUD%20Widget _asbp_character))
      (else
        (Default|SetTargetHp (Variables|/Game/Characters/Player/BP_Character.BP_Character_C|GetHUD%20Widget _asbp_character) HP HPMax))))
  (return))

(fn HaveTarget
  (return (Utilities|IsValid (Variables|Default|GetCharacterTarget))))

(fn GetDistancetoTarget
  (bind _havetarget (CallFunction|HaveTarget))
  (if _havetarget
    (return (Transformation|GetDistanceTo (Variables|Default|GetCharacterTarget) (Components|GetOwner)))))