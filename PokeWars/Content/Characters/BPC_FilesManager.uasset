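; Character component that manages Pokemon player save files on disk under the project's Characters folder.
; BeginPlay builds the paths, and SavePlayer writes each Pokemon as JSON named by its Id.
; A selected character passes to the world through a tmp file: one function copies it by Guid, another parses it back into a PokemonPlayer.
; Debug builds also save to the temp folder path itself, and the tmp-file delete is never run.
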(event EventBeginPlay
  (CallFunction|SetPathes))

(event EventTick
  (params (DeltaSeconds :type Float%20%28single-precision%29)))

(fn SetPathes
  (bind _output_get (Variables|Default|SetCharacters%20Path (Class|BlueprintPathsLibrary|Combine (Utilities|Array|MakeArray (Utilities|Paths|GetPath (Class|BlueprintPathsLibrary|ProjectDir)) "Characters"))))
  (Variables|Default|SetPlayerInfoPath (Class|BlueprintPathsLibrary|Combine (Utilities|Array|MakeArray _output_get "PlayerInfo")))
  (Variables|Default|SetCharacters%20Manager%20Path (Class|BlueprintPathsLibrary|Combine (Utilities|Array|MakeArray _output_get "CharactersManager")))
  (Variables|Default|SetAll%20CharactersPath (Class|BlueprintPathsLibrary|Combine (Utilities|Array|MakeArray _output_get "AllCharacters")))
  (Variables|Default|SetLoadToWorldTmpFilesPath (Class|BlueprintPathsLibrary|Combine (Utilities|Array|MakeArray _output_get "TmpLoadWorldFiles")))
  (return))

(fn GenereteSelectedPokemonFiletoWorld
  (params (Guid :type Guid%20Structure))
  (bind (_success _infomessage _emptytext _returnvalue) (Class|ReadandWriteFileBPLibrary|ReadStringfromFile (Class|BlueprintPathsLibrary|Combine (Utilities|Array|MakeArray (Variables|Default|GetAll%20CharactersPath) (Guid|ToString(Guid) Guid)))))
  (Development|PrintString _infomessage)
  (if _success
    (Class|ReadandWriteFileBPLibrary|SaveStringtoFile (Class|BlueprintPathsLibrary|Combine (Utilities|Array|MakeArray (Variables|Default|GetLoadToWorldTmpFilesPath) "tmp")) _returnvalue)
    (return)))

(fn LoadSelectedPokemonFiletoWorld
  (bind (_success _infomessage _emptytext _returnvalue) (Class|ReadandWriteFileBPLibrary|ReadStringfromFile (Class|BlueprintPathsLibrary|Combine (Utilities|Array|MakeArray (Variables|Default|GetLoadToWorldTmpFilesPath) "tmp"))))
  (Development|PrintString _infomessage)
  (if _success
    (bind _outjsonobject (Class|JsonBlueprintFunctionLibrary|FromString _returnvalue))
    (bind _outvalue (|GetJsonField _outjsonobject "PokemonPlayer"))
    (return (Utilities|Struct|BreakPokemonPlayerJsonModel (Utilities|Struct|MakePokemonPlayerJsonModel _outvalue)))))

(fn SavePlayer
  (params (Pokemon :type Pokemon%20Player%20Structure))
  (bind _outjsonstring (|StructtoJsonString (Utilities|Struct|MakePokemonPlayerJsonModel Pokemon)))
  (Class|ReadandWriteFileBPLibrary|SaveStringtoFile (Class|BlueprintPathsLibrary|Combine (Utilities|Array|MakeArray (Variables|Default|GetAll%20CharactersPath) (Guid|ToString(Guid) (.Id (Utilities|Struct|BreakPlayerAttributes (.PlayerAttributes (Utilities|Struct|BreakPokemonPlayer Pokemon))))))) _outjsonstring)
  (if (Class|LowEntryExtendedStandardLibrary|DebugBuild)
    (Class|ReadandWriteFileBPLibrary|SaveStringtoFile (Variables|Default|GetLoadToWorldTmpFilesPath) _outjsonstring))
  (return))