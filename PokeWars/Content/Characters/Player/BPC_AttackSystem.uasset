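; Player attack component that plays a three-step melee combo of montages on the owning BP_Character's mesh.
; IA_Attack calls Attack, which either buffers the press in SaveAttack while IsAttacking or plays the step selected by AttackIndex behind DoOnce gates.
; AttackCombo continues a buffered attack or resets the chain.
; Steps two and three share a montage, IsAttacking is never set true here, and CalculateDamage simply returns the ability's BaseDamage.
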(event Custom|Attack
  (if (Variables|Default|GetIsAttacking)
    (Variables|Default|SetSaveAttack true)
    (else
      (Variables|Default|SetSaveAttack false)
      (switch int (Variables|Default|GetAttackIndex)
        (:0
          (CallFunction|Attack1))
        (:1
          (CallFunction|Attack2))
        (:2
          (CallFunction|Attack3))))))

(event Custom|AttackCombo
  (if (Variables|Default|GetSaveAttack)
    (Variables|Default|SetSaveAttack false)
    (switch int (Variables|Default|GetAttackIndex)
      (:0
        (CallFunction|Attack1))
      (:1
        (CallFunction|Attack2))
      (:2
        (CallFunction|Attack3)))
    (else
      (CallFunction|StopCommbo))))

(event Custom|StopCommbo
  (Variables|Default|SetIsAttacking false)
  (Variables|Default|SetAttackIndex 0))

(event Custom|Attack3
  (Utilities|FlowControl|DoOnce false :!label _label
    (:Completed
      (Utilities|FlowControl|Delay 0.1)
      (Animation|Montage|PlayMontage (Variables|Default|GetCharacterMesh) "/Game/Animations/Eevee/BaseMode/Attack/AM_eevee_Anim_Attack3_Montage.AM_eevee_Anim_Attack3_Montage"
        (:then
          (Variables|Default|SetAttackIndex 3)
          (goto _label Reset))))))

(event Custom|Attack1
  (Utilities|FlowControl|DoOnce false :!label _label
    (:Completed
      (Utilities|FlowControl|Delay 0.1)
      (Animation|Montage|PlayMontage (Variables|Default|GetCharacterMesh) "/Game/Animations/Eevee/BaseMode/Attack/AM_eevee_Anim_Attack2_Montage.AM_eevee_Anim_Attack2_Montage"
        (:then
          (Variables|Default|SetAttackIndex 1)
          (goto _label Reset))))))

(event Custom|Attack2
  (Utilities|FlowControl|DoOnce false :!label _label
    (:Completed
      (Utilities|FlowControl|Delay 0.1)
      (Animation|Montage|PlayMontage (Variables|Default|GetCharacterMesh) "/Game/Animations/Eevee/BaseMode/Attack/AM_eevee_Anim_Attack3_Montage.AM_eevee_Anim_Attack3_Montage"
        (:then
          (Variables|Default|SetAttackIndex 2)
          (goto _label Reset))))))

(event Input|EnhancedActionEvents|EnhancedInputActionIA_Attack
  (params (ActionValue :type Boolean) (ElapsedSeconds :type Float%20%28double-precision%29) (TriggeredSeconds :type Float%20%28double-precision%29) (InputAction :type Input%20Action%20Object%20Reference :default "/Game/Characters/Player/Input/Actions/IA_Attack.IA_Attack"))
  (:Started
    (if (Variables|Default|GetCanAttack)
      (CallFunction|Attack))))

(event EventBeginPlay
  (bind _asbp_character (Utilities|Casting|CastToBP_Character (Components|GetOwner)))
  (Variables|Default|SetCharacterMesh (Variables|/Script/Engine.Character|GetMesh _asbp_character)))

(fn CalculateDamage
  (params (AttackId :type Guid%20Structure) (Ability :type Pokemon%20Ability%20Object%20Reference))
  (return (Variables|/Game/Structures/Structures/PokemonAbility.PokemonAbility_C|GetBaseDamage Ability)))

(fn SetCombat
  (params (IsCombat :type Boolean))
  (Variables|Default|SetIs%20Combat IsCombat)
  (return))