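; Player stats component for BP_Character that tracks health, energy, XP and level.
; On BeginPlay it waits a tick, caches the owning character and fills its HUD widget.
; Stat functions write most changes straight to the HUD, but energy gains and max-energy increases skip it; decrease functions return true on depletion.
; Reaching MaxXP carries the surplus into the next level, raises the threshold by a fixed step and plays a sound.
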(event EventBeginPlay
  (Utilities|FlowControl|DelayUntilNextTick)
  (bind _asbp_character (Utilities|Casting|CastToBP_Character (Components|GetOwner)))
  (Variables|Default|SetPlayerCharacterBP%20 _asbp_character)
  (Progress|SetPercent (Variables|/Game/UI/WB_HUD.WB_HUD_C|GetXpBar (Variables|/Game/Characters/Player/BP_Character.BP_Character_C|GetHUD%20Widget (Variables|Default|GetPlayerCharacterBP%20))) (/ (Variables|XP|GetXP) (Variables|XP|GetMaxXP)))
  (Variables|/Script/UMG.TextBlock|SetText (Variables|/Game/UI/WB_HUD.WB_HUD_C|GetXpText (Variables|/Game/Characters/Player/BP_Character.BP_Character_C|GetHUD%20Widget (Variables|Default|GetPlayerCharacterBP%20))) (Utilities|Text|FormatText "{CurrentXP} / {MaxXp}" (Variables|XP|GetXP) (Variables|XP|GetMaxXP)))
  (Rendering|Components|TextRender|SetText (Variables|/Game/UI/WB_HUD.WB_HUD_C|GetLevelText (Variables|/Game/Characters/Player/BP_Character.BP_Character_C|GetHUD%20Widget (Variables|Default|GetPlayerCharacterBP%20))) (Utilities|Text|ToText(Integer) (Variables|XP|GetLevel)))
  (Progress|SetPercent (Variables|/Game/UI/WB_HUD.WB_HUD_C|GetEnergyBar (Variables|/Game/Characters/Player/BP_Character.BP_Character_C|GetHUD%20Widget (Variables|Default|GetPlayerCharacterBP%20))) (/ (Variables|Energy|GetCurrentEnergy) (Variables|Energy|GetMaxEnergy)))
  (Rendering|Components|TextRender|SetText (Variables|/Game/UI/WB_HUD.WB_HUD_C|GetEnergyText (Variables|/Game/Characters/Player/BP_Character.BP_Character_C|GetHUD%20Widget (Variables|Default|GetPlayerCharacterBP%20))) (Utilities|Text|ToText(Float) (Variables|Energy|GetCurrentEnergy) "HalfToEven"))
  (Progress|SetPercent (Variables|/Game/UI/WB_HUD.WB_HUD_C|GetHealthBar (Variables|/Game/Characters/Player/BP_Character.BP_Character_C|GetHUD%20Widget (Variables|Default|GetPlayerCharacterBP%20))) (/ 0.0 (Variables|Health|GetMaxHealth)))
  (Rendering|Components|TextRender|SetText (Variables|/Game/UI/WB_HUD.WB_HUD_C|GetHpText (Variables|/Game/Characters/Player/BP_Character.BP_Character_C|GetHUD%20Widget (Variables|Default|GetPlayerCharacterBP%20))) (Utilities|Text|ToText(Float) (Variables|Health|GetCurrentHealth) "HalfToEven")))

(fn DecreseHealth
  (params (Damage :type Float%20%28double-precision%29))
  (bind _playercharacterbp_ (Variables|Default|GetPlayerCharacterBP%20))
  (bind _hud_widget (Variables|/Game/Characters/Player/BP_Character.BP_Character_C|GetHUD%20Widget _playercharacterbp_))
  (if (not (<= (Variables|Health|GetCurrentHealth) 0.0))
    (bind _output_get (Variables|Health|SetCurrentHealth (- (Variables|Health|GetCurrentHealth) Damage)))
    (Progress|SetPercent (Variables|/Game/UI/WB_HUD.WB_HUD_C|GetHealthBar _hud_widget) (/ _output_get (Variables|Health|GetMaxHealth)))
    (Rendering|Components|TextRender|SetText (Variables|/Game/UI/WB_HUD.WB_HUD_C|GetHpText _hud_widget) (Utilities|Text|ToText(Float) (Variables|Health|GetCurrentHealth) "HalfToEven"))
    (if (<= (Variables|Health|GetCurrentHealth) 0.0)
      _
      (else
        (return false))))
  (return true))

(fn IncreaseMaxHealth
  (params (HealthIncremention :type Float%20%28double-precision%29))
  (Variables|Health|SetMaxHealth (+ (Variables|Health|GetMaxHealth) HealthIncremention))
  (Progress|SetPercent (Variables|/Game/UI/WB_HUD.WB_HUD_C|GetHealthBar (Variables|/Game/Characters/Player/BP_Character.BP_Character_C|GetHUD%20Widget (Variables|Default|GetPlayerCharacterBP%20))) (/ (Variables|Health|GetCurrentHealth) (Variables|Health|GetMaxHealth))))

(fn DevreaseEnergy
  (params (StaminaDecrease :type Float%20%28double-precision%29))
  (bind _playercharacterbp_ (Variables|Default|GetPlayerCharacterBP%20))
  (bind _hud_widget (Variables|/Game/Characters/Player/BP_Character.BP_Character_C|GetHUD%20Widget _playercharacterbp_))
  (if (not (<= (Variables|Energy|GetCurrentEnergy) 0.0))
    (Variables|Energy|SetCurrentEnergy (- (Variables|Energy|GetCurrentEnergy) StaminaDecrease))
    (Progress|SetPercent (Variables|/Game/UI/WB_HUD.WB_HUD_C|GetEnergyBar _hud_widget) (/ (Variables|Energy|GetCurrentEnergy) (Variables|Energy|GetMaxEnergy)))
    (Rendering|Components|TextRender|SetText (Variables|/Game/UI/WB_HUD.WB_HUD_C|GetEnergyText _hud_widget) (Utilities|Text|ToText(Float) (Variables|Energy|GetCurrentEnergy) "HalfToEven"))
    (if (<= (Variables|Energy|GetCurrentEnergy) 0.0)
      _
      (else
        (return false))))
  (return true))

(fn IncreaseMaxEnergy
  (params (AddStamina :type Float%20%28double-precision%29))
  (Variables|Energy|SetMaxEnergy (+ (Variables|Energy|GetMaxEnergy) AddStamina)))

(fn IncreaseHealth
  (params (AddedHealth :type Float%20%28double-precision%29))
  (Variables|Health|SetCurrentHealth (+ (Variables|Health|GetCurrentHealth) AddedHealth))
  (if (> (Variables|Health|GetCurrentHealth) (Variables|Health|GetMaxHealth))
    (Variables|Health|SetCurrentHealth (Variables|Health|GetMaxHealth)))
  (Progress|SetPercent (Variables|/Game/UI/WB_HUD.WB_HUD_C|GetHealthBar (Variables|/Game/Characters/Player/BP_Character.BP_Character_C|GetHUD%20Widget (Variables|Default|GetPlayerCharacterBP%20))) (/ (Variables|Health|GetCurrentHealth) (Variables|Health|GetMaxHealth))))

(fn IncreaseEnergy
  (params (AddedStamina :type Float%20%28double-precision%29))
  (Variables|Energy|SetCurrentEnergy (+ (Variables|Energy|GetCurrentEnergy) AddedStamina))
  (if (> (Variables|Energy|GetCurrentEnergy) (Variables|Energy|GetMaxEnergy))
    (Variables|Energy|SetCurrentEnergy (Variables|Energy|GetMaxEnergy))))

(fn IncreaseXP
  (params (AddedXP :type Float%20%28double-precision%29))
  (Variables|XP|SetXP (+ (Variables|XP|GetXP) AddedXP))
  (if (>= (Variables|XP|GetXP) (Variables|XP|GetMaxXP))
    (LevelAndXP|IncreaseLevel 1 (- (Variables|XP|GetXP) (Variables|XP|GetMaxXP))))
  (Progress|SetPercent (Variables|/Game/UI/WB_HUD.WB_HUD_C|GetXpBar (Variables|/Game/Characters/Player/BP_Character.BP_Character_C|GetHUD%20Widget (Variables|Default|GetPlayerCharacterBP%20))) (/ (Variables|XP|GetXP) (Variables|XP|GetMaxXP)))
  (Variables|/Script/UMG.TextBlock|SetText (Variables|/Game/UI/WB_HUD.WB_HUD_C|GetXpText (Variables|/Game/Characters/Player/BP_Character.BP_Character_C|GetHUD%20Widget (Variables|Default|GetPlayerCharacterBP%20))) (Utilities|Text|FormatText "{CurrentXP} / {MaxXp}" (Variables|XP|GetXP) (Variables|XP|GetMaxXP))))

(fn IncreaseLevel
  (params (AddedLevel :type Integer) (XP :type Float%20%28double-precision%29))
  (Variables|XP|SetLevel (+ (Variables|XP|GetLevel) AddedLevel))
  (Variables|XP|SetMaxXP (+ (Variables|XP|GetMaxXP) 1.5e+02))
  (Variables|XP|SetXP XP)
  (Rendering|Components|TextRender|SetText (Variables|/Game/UI/WB_HUD.WB_HUD_C|GetLevelText (Variables|/Game/Characters/Player/BP_Character.BP_Character_C|GetHUD%20Widget (Variables|Default|GetPlayerCharacterBP%20))) (Utilities|Text|ToText(Integer) (Variables|XP|GetLevel)))
  (Audio|PlaySound2D 0 1.0 1.0 0.0 0 0))