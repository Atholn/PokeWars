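; BPC_ModeSystem is a player character component that switches between Base, Attack, Defense and Speed modes.
; On BeginPlay it casts its owner to BP_Character and caches it.
; The four arrow keys each set the Mode variable, then share a switch that swaps the character's skeletal mesh to the matching Eevee variant.
; Mode changes affect only the mesh here; no stats are modified.
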(event EventBeginPlay
  (bind _asbp_character (Utilities|Casting|CastToBP_Character (Components|GetOwner)))
  (Variables|Default|SetCharacter _asbp_character))

(event EventTick
  (params (DeltaSeconds :type Float%20%28single-precision%29)))

(event Input|KeyboardEvents|Right
  (params (Key :type Key%20Structure :default "None"))
  (bind _character (Variables|Default|GetCharacter))
  (bind _mesh (Variables|/Script/Engine.Character|GetMesh _character))
  ;[1 1 1] Switch between modes
  (:Pressed
    (Variables|Default|SetMode "NewEnumerator2")
    (switch Utilities|FlowControl|Switch|SwitchonModes (Variables|Default|GetMode)
      (:NewEnumerator0
        (Components|SkeletalMesh|SetSkeletalMeshAsset _mesh "/Game/Models/Eevee/Base/eevee.eevee"))
      (:NewEnumerator1
        (Components|SkeletalMesh|SetSkeletalMeshAsset _mesh "/Game/Models/Eevee/Attack/eeveeAttack.eeveeAttack"))
      (:NewEnumerator3
        (Components|SkeletalMesh|SetSkeletalMeshAsset _mesh "/Game/Models/Eevee/Defense/eeveeDefense.eeveeDefense"))
      (:NewEnumerator2
        (Components|SkeletalMesh|SetSkeletalMeshAsset _mesh "/Game/Models/Eevee/Speed/eeveeSpeed.eeveeSpeed")))))

(event Input|KeyboardEvents|Up
  (params (Key :type Key%20Structure :default "None"))
  (bind _character (Variables|Default|GetCharacter))
  (bind _mesh (Variables|/Script/Engine.Character|GetMesh _character))
  ;[1 1 1] Switch between modes
  (:Pressed
    (Variables|Default|SetMode "NewEnumerator0")
    (switch Utilities|FlowControl|Switch|SwitchonModes (Variables|Default|GetMode)
      (:NewEnumerator0
        (Components|SkeletalMesh|SetSkeletalMeshAsset _mesh "/Game/Models/Eevee/Base/eevee.eevee"))
      (:NewEnumerator1
        (Components|SkeletalMesh|SetSkeletalMeshAsset _mesh "/Game/Models/Eevee/Attack/eeveeAttack.eeveeAttack"))
      (:NewEnumerator3
        (Components|SkeletalMesh|SetSkeletalMeshAsset _mesh "/Game/Models/Eevee/Defense/eeveeDefense.eeveeDefense"))
      (:NewEnumerator2
        (Components|SkeletalMesh|SetSkeletalMeshAsset _mesh "/Game/Models/Eevee/Speed/eeveeSpeed.eeveeSpeed")))))

(event Input|KeyboardEvents|Left
  (params (Key :type Key%20Structure :default "None"))
  (bind _character (Variables|Default|GetCharacter))
  (bind _mesh (Variables|/Script/Engine.Character|GetMesh _character))
  ;[1 1 1] Switch between modes
  (:Pressed
    (Variables|Default|SetMode "NewEnumerator1")
    (switch Utilities|FlowControl|Switch|SwitchonModes (Variables|Default|GetMode)
      (:NewEnumerator0
        (Components|SkeletalMesh|SetSkeletalMeshAsset _mesh "/Game/Models/Eevee/Base/eevee.eevee"))
      (:NewEnumerator1
        (Components|SkeletalMesh|SetSkeletalMeshAsset _mesh "/Game/Models/Eevee/Attack/eeveeAttack.eeveeAttack"))
      (:NewEnumerator3
        (Components|SkeletalMesh|SetSkeletalMeshAsset _mesh "/Game/Models/Eevee/Defense/eeveeDefense.eeveeDefense"))
      (:NewEnumerator2
        (Components|SkeletalMesh|SetSkeletalMeshAsset _mesh "/Game/Models/Eevee/Speed/eeveeSpeed.eeveeSpeed")))))

(event Input|KeyboardEvents|Down
  (params (Key :type Key%20Structure :default "None"))
  (bind _character (Variables|Default|GetCharacter))
  (bind _mesh (Variables|/Script/Engine.Character|GetMesh _character))
  ;[1 1 1] Switch between modes
  (:Pressed
    (Variables|Default|SetMode "NewEnumerator3")
    (switch Utilities|FlowControl|Switch|SwitchonModes (Variables|Default|GetMode)
      (:NewEnumerator0
        (Components|SkeletalMesh|SetSkeletalMeshAsset _mesh "/Game/Models/Eevee/Base/eevee.eevee"))
      (:NewEnumerator1
        (Components|SkeletalMesh|SetSkeletalMeshAsset _mesh "/Game/Models/Eevee/Attack/eeveeAttack.eeveeAttack"))
      (:NewEnumerator3
        (Components|SkeletalMesh|SetSkeletalMeshAsset _mesh "/Game/Models/Eevee/Defense/eeveeDefense.eeveeDefense"))
      (:NewEnumerator2
        (Components|SkeletalMesh|SetSkeletalMeshAsset _mesh "/Game/Models/Eevee/Speed/eeveeSpeed.eeveeSpeed")))))