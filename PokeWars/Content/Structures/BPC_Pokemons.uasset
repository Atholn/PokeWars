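; BPC_Pokemons is a component that holds the game's Pokémon roster and exposes it through GetPokemons.
; BeginPlay fills the Pokemons array with hardcoded structs carrying ID, name, description, type, and base, attack, defense and speed profile images and meshes.
; Jolteon and Vaporeon are populated but share the same parsed GUID.
; The Flareon add has no item wired, leaving its struct and separate GUID unused.
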(event EventBeginPlay
  (bind _returnvalue (Utilities|Enum|LiteralenumPokemonEnum "NewEnumerator1"))
  (bind _returnvalue_2 (Utilities|Enum|LiteralenumPokemonEnum "NewEnumerator2"))
  (bind _pokemons (Variables|Default|GetPokemons))
  ;[1 1 1] Jolteon
  (Utilities|Array|Add _pokemons (Utilities|Struct|MakePokemon (.OutGuid (Class|KismetGuidLibrary|ParseStringtoGuid "3ab58d56-b26f-4a1e-bf00-57025d9dd7ad")) (Utilities|String|EnumtoString _returnvalue) "Jolteon Description" _returnvalue "NewEnumerator0" "" (Utilities|Struct|MakeProfileImages "/Game/UI/CharactersMenu/PokemonProfileImages/JolteonProfileImage.JolteonProfileImage" "/Game/UI/CharactersMenu/PokemonProfileImages/JolteonAttackProfile-Photoroom.JolteonAttackProfile-Photoroom" "/Game/UI/CharactersMenu/PokemonProfileImages/JolteonDefenseProfile.JolteonDefenseProfile" "/Game/UI/CharactersMenu/PokemonProfileImages/JolteonSpeedProfile.JolteonSpeedProfile") (Utilities|Struct|MakePokemonMeshes "/Game/Models/Jolteon/Base/JolteonBase.JolteonBase" "/Game/Models/Jolteon/Attack/JolteonAttack.JolteonAttack" "/Game/Models/Jolteon/Defense/JolteonDefense.JolteonDefense" "/Game/Models/Jolteon/Speed/JolteonSpeed.JolteonSpeed")))
  ;[1 1 1] Flareon
  (Utilities|Array|Add :TargetArray _pokemons)
  ;[1 1 1] Vaporeon
  (Utilities|Array|Add _pokemons (Utilities|Struct|MakePokemon (.OutGuid (Class|KismetGuidLibrary|ParseStringtoGuid "3ab58d56-b26f-4a1e-bf00-57025d9dd7ad")) (Utilities|String|EnumtoString _returnvalue_2) "Vaporeon Description" _returnvalue_2 "NewEnumerator2" "" (Utilities|Struct|MakeProfileImages "/Game/UI/CharactersMenu/PokemonProfileImages/VaporeonProfileImage.VaporeonProfileImage" "/Game/UI/CharactersMenu/PokemonProfileImages/VaporeonAttackProfile.VaporeonAttackProfile" "/Game/UI/CharactersMenu/PokemonProfileImages/VaporeonDefenseProfile.VaporeonDefenseProfile" "/Game/UI/CharactersMenu/PokemonProfileImages/VaporeonSpeedProfile.VaporeonSpeedProfile") (Utilities|Struct|MakePokemonMeshes "/Game/Models/Vaporeon/Base/VaporeonBase.VaporeonBase" "/Game/Models/Vaporeon/Attack/VaporeonAttack.VaporeonAttack" "/Game/Models/Vaporeon/Defense/VaporeonDefense.VaporeonDefense" "/Game/Models/Vaporeon/Speed/VaporeonSpeed.VaporeonSpeed"))))

(fn GetPokemons
  (return (Variables|Default|GetPokemons)))